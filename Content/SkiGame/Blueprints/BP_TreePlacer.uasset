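; BP_TreePlacer scatters trees at random through a box volume in the ski game.
; Its construction script adds instances to one InstancedStaticMesh at random points in the Box extent, with the count driven by NumberOfTrees.
; Each world-space point is rotated by a fixed angle about the actor's right axis, pivoting on the world origin rather than the actor.
; Instances share the actor's rotation and a fixed uniform scale.
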(fn `UserConstructionScript`
  (for _ (range (+ (`self.NumberOfTrees`) 1))
    (`InstancedStaticMeshComponent.AddInstanceWorldSpace` (`self.InstancedStaticMesh`) (`KismetMathLibrary.MakeTransform` (`KismetMathLibrary.RotateAngleAxis` (`KismetMathLibrary.RandomPointInBoundingBox` (`self.K2_GetActorLocation`) (`BoxComponent.GetScaledBoxExtent` (`self.Box`))) 20.0 (`self.GetActorRightVector`)) (`self.K2_GetActorRotation`) (5.0 5.0 5.0)))))