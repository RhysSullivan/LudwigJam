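; Skier actor with two independently steered skis, moved down a slope by custom velocity math rather than physics.
; Each input axis turns one ski within a yaw limit, rotating its velocity alongside.
; Per tick, skis accelerate by downhill alignment and brake when angled inward like a snowplow; diverging velocities also trigger corrective rotation.
; The averaged ski velocities move the player without sweep and yaw the body toward travel.
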(event `self.ReceiveBeginPlay`
  (bind _output_get (set `self.DownhillDirection` (`self.GetActorForwardVector`)))
  (bind _output_get_2 (set `self.Velocity` (* _output_get (`self.StartSpeed`))))
  (bind _output_get_3 (set `self.LeftSkiVelocity` _output_get_2))
  (set `self.RightSkiVelocity` _output_get_3))

(event `self.ReceiveTick`
  (params (DeltaSeconds :type "Float (single-precision)"))
  (bind _returnvalue (`KismetMathLibrary.Dot_VectorVector` (`KismetMathLibrary.Normal` (`self.LeftSkiVelocity`)) (`KismetMathLibrary.Normal` (`self.RightSkiVelocity`))))
  (bind _returnvalue_2 (- _returnvalue 1.0))
  (set `self.FrameTime` DeltaSeconds)
  (`self.UpdatePlayerLocation` DeltaSeconds)
  (`self.UpdateSkiRotationAndLocation` DeltaSeconds)
  (bind _newvelocity (`self.UpdateSkiForce` (`self.LeftSkiVelocity`) DeltaSeconds))
  (set `self.LeftSkiVelocity` _newvelocity)
  (bind _newvelocity_2 (`self.UpdateSkiForce` (`self.RightSkiVelocity`) DeltaSeconds))
  (set `self.RightSkiVelocity` _newvelocity_2)
  (if (and (< _returnvalue 0.95) (> _returnvalue 0.0))
    (bind (_newvelocity_3 _newangle) (`self.ForceSkiRotation` _returnvalue_2 (`self.LeftSkiVelocity`) (`self.LeftSkiRotation`)))
    (set `self.LeftSkiVelocity` _newvelocity_3)
    (set `self.LeftSkiRotation` _newangle)
    (bind (_newvelocity_4 _newangle_2) (`self.ForceSkiRotation` (* _returnvalue_2 -1.0) (`self.RightSkiVelocity`) (`self.RightSkiRotation`)))
    (set `self.RightSkiVelocity` _newvelocity_4)
    (set `self.RightSkiRotation` _newangle_2)))

(event `InputAxis|RotateRightSki`
  (params (AxisValue :type "Float (single-precision)"))
  (bind (_skirotation _newvelocity) (`self.DoSkiRotationMath` AxisValue (`self.RightSkiRotation`) (`self.RightSkiVelocity`)))
  (set `self.RightSkiRotation` _skirotation)
  (set `self.RightSkiVelocity` _newvelocity))

(event `InputAxis|RotateLeftSki`
  (params (AxisValue :type "Float (single-precision)"))
  (bind (_skirotation _newvelocity) (`self.DoSkiRotationMath` AxisValue (`self.LeftSkiRotation`) (`self.LeftSkiVelocity`)))
  (set `self.LeftSkiRotation` _skirotation)
  (set `self.LeftSkiVelocity` _newvelocity))

(fn `DoSkiRotationMath`
  (params (Axis :type "Float (double-precision)") (CurrentSkiVal :type "Float (double-precision)") (CurrentVelocity :type "Vector Structure"))
  (returns (SkiRotation :type "Float (double-precision)") (NewVelocity :type "Vector Structure"))
  (bind _maxskirotation (`self.MaxSkiRotation`))
  (bind _returnvalue (`KismetMathLibrary.ClampAngle` (+ (* (* Axis (`self.SkiTurnRate`)) (`GameplayStatics.GetWorldDeltaSeconds`)) CurrentSkiVal) (* _maxskirotation -1.0) _maxskirotation))
  (return _returnvalue (`KismetMathLibrary.RotateAngleAxis` (`local.CurrentVelocity`) (- _returnvalue (`local.CurrentSkiVal`)) (`self.GetActorUpVector`))))

(fn `ForceSkiRotation`
  (params (Delta :type "Float (double-precision)") (Velocity :type "Vector Structure") (SkiRotation :type "Float (double-precision)"))
  (returns (NewVelocity :type "Vector Structure") (NewAngle :type "Float (double-precision)") (Break :type Boolean))
  (bind _maxskirotation (`self.MaxSkiRotation`))
  (bind _returnvalue (`KismetMathLibrary.ClampAngle` (+ (`local.SkiRotation`) (* Delta (* 100.0 (`self.FrameTime`)))) (* _maxskirotation -1.0) _maxskirotation))
  (return (`KismetMathLibrary.RotateAngleAxis` Velocity (- _returnvalue (`local.SkiRotation`)) (`self.GetActorUpVector`)) _returnvalue false))

(fn `UpdatePlayerLocation`
  (params (DeltaTime :type "Float (double-precision)"))
  (bind _body (`self.Body`))
  (bind _velocity (`self.Velocity`))
  (bind (_returnvalue_roll _returnvalue_pitch _returnvalue_yaw) (`KismetMathLibrary.BreakRotator` (`KismetMathLibrary.MakeRotFromX` _velocity)))
  (bind (_relativerotation_roll _relativerotation_pitch) (`KismetMathLibrary.BreakRotator` (`SceneComponent.RelativeRotation` _body)))
  (bind _output_get (set `self.Velocity` (* (/ (+ (`self.LeftSkiVelocity`) (`self.RightSkiVelocity`)) 2.0) DeltaTime)))
  (`SceneComponent.K2_AddWorldOffset` (`self.Player`) _output_get false false)
  (if (> (`KismetMathLibrary.VSizeSquared` _velocity) 1.0)
    (`SceneComponent.K2_SetRelativeRotation` _body (`KismetMathLibrary.MakeRotator` _relativerotation_roll _relativerotation_pitch _returnvalue_yaw) false false)))

(fn `UpdateSkiForce`
  (params (SkiVelocity :type "Vector Structure") (DT :type "Float (double-precision)"))
  (returns (NewVelocity :type "Vector Structure"))
  (return (+ (+ (* (`KismetMathLibrary.Normal` (`local.SkiVelocity`)) (* (`KismetMathLibrary.FClamp` (- (`KismetMathLibrary.Dot_VectorVector` (`KismetMathLibrary.Normal` (`self.DownhillDirection`)) (`KismetMathLibrary.Normal` (`local.SkiVelocity`))) 0.5) 0.1 0.6) (* (`self.DownhillAcceleration`) (`local.DT`)))) (* (* (`KismetMathLibrary.Normal` (`local.SkiVelocity`)) -1.0) (`KismetMathLibrary.Abs` (* (`KismetMathLibrary.FClamp` (- (`self.RightSkiRotation`) (`self.LeftSkiRotation`)) -100.0 0.0) (* (* (`local.DT`) 70.0) (`KismetMathLibrary.FClamp` (`KismetMathLibrary.VSizeSquared` (`local.SkiVelocity`)))))))) (`local.SkiVelocity`))))

(fn `UpdateSkiRotationAndLocation`
  (params (DeltaTime :type "Float (double-precision)"))
  (`SceneComponent.K2_SetRelativeRotation` (`self.SkiLeft`) (`KismetMathLibrary.MakeRotator` 0.0 0.0 (+ (`self.LeftSkiRotation`) 0.0)) false false)
  (`SceneComponent.K2_SetRelativeRotation` (`self.SkiRight`) (`KismetMathLibrary.MakeRotator` 0.0 0.0 (+ (`self.RightSkiRotation`) 0.0)) false false))

(fn `UserConstructionScript`)